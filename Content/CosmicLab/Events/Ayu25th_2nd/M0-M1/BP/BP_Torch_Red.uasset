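; Red torch actor pairing a PointLight with a Niagara effect, starting lit or unlit via StartOn.
; TurnOn plays a timeline that fades the light in, activates Niagara once, then calls TurnOff after TimerToTurnOff.
; TurnOff reverses the timeline, deactivating Niagara and resetting the DoOnce when finished.
; Construction applies LightIntensity, drop amount and zero flicker, but runtime intensity uses a hard-coded peak.
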(event Custom|TurnOn
  (if (not (Variables|Default|GetisOn))
    (bind (_direction _0to1) (Timeline|Tween PlayFromStart)
      (:Update
        (Rendering|Components|Light|SetIntensity (Variables|Default|GetPointLight) (* _0to1 2e+03))
        (switch Utilities|FlowControl|Switch|SwitchonETimelineDirection _direction
          (:Forward
            (Utilities|FlowControl|DoOnce false :!label _label
              (:Completed
                (Components|Activation|Activate (Variables|Default|GetNiagara) true)
                (Variables|Default|SetisOn true)
                (Utilities|FlowControl|Delay (Variables|Default|GetTimerToTurnOff))
                (CallFunction|TurnOff))))))
      (:Finished
        (switch Utilities|FlowControl|Switch|SwitchonETimelineDirection _direction
          (:Backward
            (Components|Activation|Deactivate (Variables|Default|GetNiagara))
            (Variables|Default|SetisOn false)
            (goto _label Reset)))))))

(event Custom|TurnOff
  (bind (_direction _0to1) (Timeline|Tween ReverseFromEnd)
    (:Update
      (Rendering|Components|Light|SetIntensity (Variables|Default|GetPointLight) (* _0to1 2e+03))
      (switch Utilities|FlowControl|Switch|SwitchonETimelineDirection _direction
        (:Forward
          (Utilities|FlowControl|DoOnce false :!label _label
            (:Completed
              (Components|Activation|Activate (Variables|Default|GetNiagara) true)
              (Variables|Default|SetisOn true)
              (Utilities|FlowControl|Delay (Variables|Default|GetTimerToTurnOff))
              (CallFunction|TurnOff))))))
    (:Finished
      (switch Utilities|FlowControl|Switch|SwitchonETimelineDirection _direction
        (:Backward
          (Components|Activation|Deactivate (Variables|Default|GetNiagara))
          (Variables|Default|SetisOn false)
          (goto _label Reset))))))

(event EventBeginPlay
  (if (Variables|Default|GetStartOn)
    (Rendering|Components|Light|SetIntensity (Variables|Default|GetPointLight) 2e+03)
    (Components|Activation|SetAutoActivate (Variables|Default|GetNiagara) true)
    (else
      (Rendering|Components|Light|SetIntensity (Variables|Default|GetPointLight) 0.0)
      (Components|Activation|SetAutoActivate (Variables|Default|GetNiagara) false))))

(fn ConstructionScript
  (Effects|Components|ParticleSystem|SetFloatParameter (Variables|Default|GetNiagara) "User.Flickering" 0.0)
  (Effects|Components|ParticleSystem|SetFloatParameter (Variables|Default|GetNiagara) "User.DropsAmmount" (Variables|Default|GetDropsAmmount))
  (Rendering|Components|Light|SetIntensity (Variables|Default|GetPointLight) (Variables|Default|GetLight%20Intensity)))