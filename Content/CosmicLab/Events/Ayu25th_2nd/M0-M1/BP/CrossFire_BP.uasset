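; CrossFire_BP is an event prop that dissolves a Cross mesh and sets a fire effect on it for a timed span.
; On BeginPlay a timeline drives the materials' Dissolve Amount, then activates CrossFireFX when it finishes.
; In parallel, a fixed delay of about a minute leads to a second timeline played in reverse from its end, which drives the same parameter and deactivates the effect on completion.
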(event EventBeginPlay
  (Utilities|FlowControl|Sequence
    (:then_0
      (Components|Activation|Deactivate (Variables|Default|GetCrossFireFX))
      (Rendering|Material|SetScalarParameterValueonMaterials (Variables|Default|GetCross) "Dissolve Amount" 0.0)
      (bind _dissolveamount (Timeline|Timeline Play)
        (:Update
          (Rendering|Material|SetScalarParameterValueonMaterials (Variables|Default|GetCross) "Dissolve Amount" _dissolveamount))
        (:Finished
          (Components|Activation|Activate (Variables|Default|GetCrossFireFX) false))))
    (:then_1
      (Utilities|FlowControl|Delay 63.0)
      (bind _dissolveamount_2 (Timeline|Timeline_0 ReverseFromEnd)
        (:Update
          (Rendering|Material|SetScalarParameterValueonMaterials (Variables|Default|GetCross) "Dissolve Amount" _dissolveamount_2))
        (:Finished
          (Components|Activation|Deactivate (Variables|Default|GetCrossFireFX)))))))

(event EventTick
  (params (DeltaSeconds :type Float%20%28single-precision%29)))

(fn ConstructionScript)